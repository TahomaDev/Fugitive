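; Player character Blueprint that handles melee attack animation and item gathering.
; Melee plays a random montage; gathering walks to distant pickups or plays a montage that locks movement and attacking, adding the item to inventory on completion.
; OnGatheringCPP skips the distance check; the arrival check and noise report are disconnected, leaving Tick and the looping noise timer's event empty.
; A debug G key equips a grenade.
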(event `self.ReceiveBeginPlay`
  (`KismetSystemLibrary.K2_SetTimerDelegate` (delegate `NoiseEvent`) 1.0 true))

(event `NoiseEvent`)

(event `Key|G`
  (params (Key :type "Key Structure"))
  ;[1 0.5156 0] Debug
  (:`Pressed`
    (`self.CharacterInitWeapon` "Grenade_v1")))

(event `self.ReceiveTick`
  (params (DeltaSeconds :type "Float (single-precision)"))
  ;[0.3594 0 1] EventTick
)

(event `self.OnHandAttack`
  ;[0.8281 0 1] Melee attack
  (`|PlayMontage` (`self.Mesh`) (`|GetArrayItem` (`self.Meele Attack`) (`KismetMathLibrary.RandomIntegerInRange` 0 (- (`KismetArrayLibrary.Array_Length` (`self.Meele Attack`)) 1)))
    (:`OnCompleted`
      (set `self.bCanAttack` true))))

(event `self.OnGathering`
  (params (ItemInfo :type "ItemInfo Structure") (TargetActor :type "Actor Object Reference"))
  (`parent.OnGathering` ItemInfo TargetActor)
  (`self.OnGathering1` ItemInfo TargetActor))

(event `OnGathering1`
  (params (ItemInfo :type "ItemInfo Structure") (PickupActor :type "Actor Object Reference"))
  ;[1 0 0.2109] On Gathering
  (set `self.bIsGathering` true)
  (set `self.GatheringInfo` ItemInfo)
  (if (> (`KismetMathLibrary.VSize` (- (`self.K2_GetActorLocation` PickupActor) (`self.K2_GetActorLocation`))) (`self.MinDistanceToInteractActor`))
    ;;[0.3828 1 0] Move to actor
    (set `self.GatheringActor` PickupActor)
    (bind _asfugitive_player_controller (cast `FugitivePlayerController` (`self.GetController`)))
    (`AIBlueprintHelperLibrary.SimpleMoveToActor` _asfugitive_player_controller (`self.GatheringActor`))
    (else
      (set `self.GatheringActor` null)
      (`|PlayMontage` (`self.Mesh`) "/Game/_NOGIT/MY/Anim/2/Gathering_Objects_Montage.Gathering_Objects_Montage" :!label _label
        (:`then`
          (set `self.bCanAttack` false)
          (bind _asfugitive_player_controller_2 (cast `FugitivePlayerController` (`self.GetOwner`)))
          (`FugitivePlayerController.SetCanMove` _asfugitive_player_controller_2 false))
        (:`OnCompleted`
          (bind _returnvalue (`self.GetInventory`))
          (bind _returnvalue_2 (`T_InventoryComponent.AddItem` _returnvalue (stale `self.OnGatheringCPP` ItemInfo) 0))
          (message `IObjectReact.SetAmount` (stale `self.OnGatheringCPP` TargetActor) null (`KismetMathLibrary.Conv_IntToByte` _returnvalue_2))
          (set `self.bCanAttack` true :!label _label_2)
          (set `self.bIsGathering` false)
          (bind _asfugitive_player_controller_3 (cast `FugitivePlayerController` (`self.GetOwner`)))
          (`FugitivePlayerController.SetCanMove` _asfugitive_player_controller_3 true))
        (:`OnInterrupted`
          (goto _label_2))))))

(event `self.OnGatheringCPP`
  (params (ItemInfo :type "ItemInfo Structure") (TargetActor :type "Actor Object Reference"))
  ;[1 0 0.2109] On Gathering
  (goto _label))

(fn `UserConstructionScript`)