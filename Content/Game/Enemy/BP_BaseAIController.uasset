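; Base enemy AI controller that enables perception and runs BT_AIBase when a tagged player comes within activation range.
; A looping timer checks cached players for activation, then starts another that disables senses and stops logic for any out-of-range player, restarting the activation timer every pass without clearing itself.
; Perception updates write player hearing and other senses' results to the blackboard, saving the last known location with debug drawing on target loss.
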(event `RunTimerByBehaviorStart`
  (bind _returnvalue (`KismetSystemLibrary.K2_SetTimerDelegate` (delegate `CheckDistanceToPlayer`) 3.0 true :!label _label))
  (set `self.CheckStartAI_HeaderTimer` _returnvalue))

(event `self.ReceiveBeginPlay`
  (`self.SetPerceptionActive` false)
  (bind _outactors (`GameplayStatics.GetAllActorsWithTag` "Player")) ; Нужен массив игроков, чтобы не искать акторы
  (set `self.PlayersList` _outactors)
  (goto _label))

(event `CheckDistanceToPlayer`
  ;[1 0.6094 0] Activate AI
  (for _array_element (`self.PlayersList`)
    (if (< (`self.GetDistanceTo` _array_element self) (`self.MaxDistanceFromActivateAI`))
      (`self.SetPerceptionActive` true)
      (`self.RunBehaviorTree` "/Game/Game/Enemy/BT/BT_AIBase.BT_AIBase")
      (`KismetSystemLibrary.K2_ClearAndInvalidateTimerHandle` (`self.CheckStartAI_HeaderTimer`))
      (set `self.CheckStartAI_HeaderTimer` (struct))
      (bind _returnvalue (`KismetSystemLibrary.K2_SetTimerDelegate` (delegate `CustomEvent_0`) 5.0 true))
      (set `self.CheckEndAI_HeaderTimer` _returnvalue))))

(event `CustomEvent_0`
  ;[1 0 0.2812] Deactivate AI
  (bind _outactors (`GameplayStatics.GetAllActorsWithTag` "Player")) ; Нужен массив игроков, чтобы не искать акторы
  (for _array_element _outactors
    (if (> (`self.GetDistanceTo` _array_element self) (`self.MaxDistanceFromActivateAI`))
      (`self.SetPerceptionActive` false)
      (`BrainComponent.StopLogic` (`self.BrainComponent`) "")))
  (`self.RunTimerByBehaviorStart`))

(event `self.AIPerception.OnTargetPerceptionUpdated`
  (params (Actor :type "Actor Object Reference") (Stimulus :type "AIStimulus Structure"))
  (bind _returnvalue (`AIBlueprintHelperLibrary.GetBlackboard` null))
  (bind _returnvalue_2 (`AIBlueprintHelperLibrary.GetBlackboard` null))
  (bind _returnvalue_3 (`AIBlueprintHelperLibrary.GetBlackboard` null))
  (bind _currenttarget (`self.CurrentTarget`))
  (bind _currenttarget_2 (`self.CurrentTarget`))
  (bind _returnvalue_4 (`self.K2_GetActorLocation` (`self.CurrentTarget`)))
  (`/Engine/EditorBlueprintResources/StandardMacros.IsValid` Actor
    (:`Is Valid`
      (set `self.CurrentTarget` Actor)
      (if (`self.ActorHasTag` Actor "Player")
        (bind _returnvalue_5 (`AIPerceptionSystem.GetSenseClassForStimulus` Stimulus))
        (if (== _returnvalue_5 "/Script/AIModule.AISense_Hearing")
          (`/Engine/EditorBlueprintResources/StandardMacros.IsValid` _currenttarget_2
            (:`Is Valid`
              (`BlackboardComponent.SetValueAsVector` _returnvalue "BB_LastTargetVector" (`self.K2_GetActorLocation` _currenttarget_2))
              (`BlackboardComponent.SetValueAsBool` _returnvalue "BB_CanHearTarget" true)))
          (elif (`.bSuccessfullySensed` (break `AIStimulus` Stimulus))
            (`/Engine/EditorBlueprintResources/StandardMacros.IsValid` _currenttarget
              (:`Is Valid`
                (`BlackboardComponent.SetValueAsObject` _returnvalue_2 "BB_TargetActor" _currenttarget)
                (`BlackboardComponent.SetValueAsVector` _returnvalue_2 "BB_TargetVector" (`self.K2_GetActorLocation` _currenttarget))
                (`BlackboardComponent.SetValueAsBool` _returnvalue_2 "BB_CanSeeTarget" true)))
            (else
              (`/Engine/EditorBlueprintResources/StandardMacros.IsValid` (`self.CurrentTarget`)
                (:`Is Valid`
                  (`/Engine/EditorBlueprintResources/StandardMacros.IsValid` (`self.CurrentTarget`)
                    (:`Is Valid`
                      (`BlackboardComponent.SetValueAsObject` _returnvalue_3 "BB_TargetActor" null)
                      (`BlackboardComponent.SetValueAsVector` _returnvalue_3 "BB_TargetVector" (0.0 0.0 0.0))
                      (`BlackboardComponent.SetValueAsBool` _returnvalue_3 "BB_CanSeeTarget" false)
                      (`BlackboardComponent.SetValueAsVector` _returnvalue_3 "BB_LastTargetVector" _returnvalue_4)
                      (`KismetSystemLibrary.DrawDebugSphere` _returnvalue_4 10.0 12 (struct :`R` 0.126427 :`G` 0.138753 :`B` 1.0 :`A` 1.0) 10.0)
                      (`KismetSystemLibrary.DrawDebugString` _returnvalue_4 "I lost target here" null (struct :`A` 1.0) 10.0))
                    (:`Is Not Valid`
                      (`KismetSystemLibrary.PrintString` "Perseption: Current Target invalid" true true (struct :`R` 1.0 :`G` 0.057227 :`A` 1.0)))))))))))
    (:`Is Not Valid`
      (`BlackboardComponent.SetValueAsObject` (`AIBlueprintHelperLibrary.GetBlackboard` null) "BB_TargetActor" null))))

(fn `SetPerceptionActive`
  (params (Active :type Boolean))
  (bind _aiperception (`self.AIPerception`))
  (`AIPerceptionComponent.SetSenseEnabled` _aiperception "/Script/AIModule.AISense_Hearing" Active)
  (`AIPerceptionComponent.SetSenseEnabled` _aiperception "/Script/AIModule.AISense_Damage" Active)
  (`AIPerceptionComponent.SetSenseEnabled` _aiperception "/Script/AIModule.AISense_Sight" Active))

(fn `StartBehaviorTree`
  (`self.RunBehaviorTree` "/Game/Game/Enemy/BT/BT_AIBase.BT_AIBase")
  (`BlackboardComponent.SetValueAsEnum` (`AIBlueprintHelperLibrary.GetBlackboard` null) "BB_ChaseState" 3))

(fn `UserConstructionScript`)