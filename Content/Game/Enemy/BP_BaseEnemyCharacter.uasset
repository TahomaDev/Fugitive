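; Base enemy character that provides melee, firearm and grenade attacks, plus queries for team identity, movement, attack readiness and fire range.
; Attack events lock CanAttackPawn until their montage completes, or a fixed delay for firing, and weapon slots switch by attack type or target distance.
; GrenadeAttack stores the target for a separate OnGrenadeFire event that launches the grenade.
; Damage plays random hit montages that pause attacking and movement; empty health removes the radar marker.
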(event `self.OnEmptyHealtBP`
  (`T_MinimapObject.RemoveFromRadar` (`self.T_MinimapObject`)))

(event `/Game/Game/Enemy/BPI_Combat.HandAttack`
  (bind _handattackanims (`self.HandAttackAnims`))
  ;[1 0 0.8906] Hand attack
  (set `self.bCanAttackPawn` false)
  (`self.TakeSelectWeapon` 0)
  (`|PlayMontage` (`self.Mesh`) (`|GetArrayItem` _handattackanims (`KismetMathLibrary.RandomIntegerInRange` 0 (- (`KismetArrayLibrary.Array_Length` _handattackanims) 1))) ; Анимация атаки
    (:`OnCompleted`
      (set `self.bCanAttackPawn` true))))

(event `/Game/Game/Enemy/BPI_Combat.ChangeWeapon`
  (params (DistanceToTarget :type "Float (single-precision)"))
  ;[0.3828 0 1] Change weapon
  (if (< DistanceToTarget (`self.FireDistanceMin`))
    (`self.TakeSelectWeapon` 0)
    (else
      (`self.TakeSelectWeapon` 1))))

(event `/Game/Game/Enemy/BPI_Combat.FireAttack`
  (params (TargetActor :type "Actor Object Reference"))
  ;[0.1484 1 0] Fire attack
  (set `self.bCanAttackPawn` false)
  (`self.TakeSelectWeapon` 1)
  (`self.WeaponFire` TargetActor)
  (`KismetSystemLibrary.Delay` 2.0) ; Это заместо анимации тут
  (set `self.bCanAttackPawn` true))

(event `/Game/Game/Enemy/BPI_Combat.GrenadeAttack`
  (params (TargetActor :type "Actor Object Reference"))
  ;[0 0.4375 1] Grenade attack
  (set `self.bCanAttackPawn` false)
  (set `self.TargetActor` TargetActor)
  (`|PlayMontage` (`self.Mesh`) (`self.GrenadeThrowAnim`)
    (:`OnCompleted`
      (set `self.bCanAttackPawn` true))))

(event `self.ReceiveAnyDamage`
  (params (Damage :type "Float (single-precision)") (DamageType :type "DamageType Object Reference") (InstigatedBy :type "Controller Object Reference") (DamageCauser :type "Actor Object Reference"))
  (bind _hitanimation (`self.HitAnimation`))
  (bind _returnvalue (`KismetArrayLibrary.Array_Length` _hitanimation))
  (bind _output (`|GetArrayItem` _hitanimation (`KismetMathLibrary.RandomIntegerInRange` 0 (- _returnvalue 1))))
  ;[1 0 0.6797] AnyDamage
  (if (> _returnvalue 0)
    (if (and (`KismetSystemLibrary.IsValid` _output) (!= _output null))
      (set `self.bCanAttackPawn` false)
      (`self.SetCanMove` false)
      (`|PlayMontage` (`self.Mesh`) _output
        (:`OnCompleted`
          (set `self.bCanAttackPawn` true)
          (`self.SetCanMove` true))))))

(event `OnGrenadeFire`
  ;[0 0.4375 1] Grenade attack
  (`self.TakeSelectWeapon` 2)
  (`self.GrenadeFire` (`self.TargetActor`)))

(fn `CanFireAttack`
  (params (EnemyLocation :type "Vector Structure"))
  (returns (`CanAttack?` :type Boolean))
  (bind _returnvalue (`self.CanFireAttackPawn` EnemyLocation))
  (return _returnvalue))

(fn `CanHandAttack`
  (returns (`CanAttack?` :type Boolean))
  (return (`self.bCanAttackPawn`)))

(fn `CanMove`
  (returns (`CanMove?` :type Boolean))
  (bind _returnvalue (`self.GetCanMove`))
  (return _returnvalue))

(fn `CanThrowGrenadeAttack`
  (params (TargetActor :type "Actor Object Reference"))
  (returns (Result :type Boolean))
  (bind _returnvalue (`self.CanThrowGrenade` TargetActor))
  (return _returnvalue))

(fn `GetFireDistance`
  (returns (Min :type "Float (double-precision)") (Max :type "Float (double-precision)") (CanFire :type Boolean))
  (return (`self.FireDistanceMin`) (`self.FireDistanceMax`) (== (`self.CurrentWeaponSlot`) 1)))

(fn `HowAreYou`
  (params (Actor :type "Actor Object Reference"))
  (returns (ReturnValue :type "EObjectAction Enum"))
  (return "Enemy"))

(fn `UserConstructionScript`)