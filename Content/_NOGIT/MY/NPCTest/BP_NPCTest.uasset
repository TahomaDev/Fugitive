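; BP_NPCTest is a test NPC Blueprint that supplies a single-use interaction response.
; HowAreYou returns InteractNPC on the first call and sets IsUsed, so every later call returns None.
; The other interaction query functions are minimal: zero interact time with a false result, no custom depth for selection, and an empty WhatIGet.
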(fn `GetInteractTime`
  (returns (Time :type "Float (double-precision)") (ReturnValue :type Boolean))
  (return 0.0 false))

(fn `HaveYouCustomDephForSelect`
  (returns (ReturnValue :type Boolean))
  (return false))

(fn `HowAreYou`
  (params (Actor :type "Actor Object Reference"))
  (returns (ReturnValue :type "EObjectAction Enum"))
  (locals (bLocalIsUsed :type Boolean))
  (bind _output_get (set `local.bLocalIsUsed` (`self.bIsUsed`)))
  (set `self.bIsUsed` true)
  (return (select `bool` _output_get :`false` "InteractNPC" :!type "EObjectAction Enum")))

(fn `UserConstructionScript`)

(fn `WhatIGet`
  (params (Actor :type "Actor Object Reference"))
  (returns (ReturnValue :type "ItemInfo Structure"))
  (return))