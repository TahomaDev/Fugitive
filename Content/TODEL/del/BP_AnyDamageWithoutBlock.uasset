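; BP_AnyDamageWithoutBlock is a damage volume that hurts the player with unblockable generic damage.
; Its Box overlap stores the BP_Player and sets a damage flag, and any component leaving the box clears both.
; While flagged, each Tick disables block chance on the player's HealthComponent and applies a small fixed damage, so the rate follows frame rate.
; Block chance is not re-enabled here.
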(event `self.ReceiveTick`
  (params (DeltaSeconds :type "Float (single-precision)"))
  (bind _as_bp_player (`self.As BP Player`))
  (if (`self.bIsDamaged`)
    (`/Engine/EditorBlueprintResources/StandardMacros.IsValid` _as_bp_player
      (:`Is Valid`
        (`T_HealthComponent.EnableBlockChanse` (`FugitiveCharacter.HealthComponent` _as_bp_player) false)
        (`GameplayStatics.ApplyDamage` _as_bp_player 1.0)))))

(event `self.Box.OnComponentBeginOverlap`
  (params (OverlappedComponent :type "PrimitiveComponent Object Reference") (OtherActor :type "Actor Object Reference") (OtherComp :type "PrimitiveComponent Object Reference") (OtherBodyIndex :type Integer) (bFromSweep :type Boolean) (SweepResult :type "HitResult Structure (by ref)"))
  (bind _asbp_player (cast `/Game/Game/Player/BP_Player` OtherActor))
  (set `self.As BP Player` _asbp_player)
  (set `self.bIsDamaged` true))

(event `self.Box.OnComponentEndOverlap`
  (params (OverlappedComponent :type "PrimitiveComponent Object Reference") (OtherActor :type "Actor Object Reference") (OtherComp :type "PrimitiveComponent Object Reference") (OtherBodyIndex :type Integer))
  (set `self.As BP Player` null)
  (set `self.bIsDamaged` false))

(fn `UserConstructionScript`)